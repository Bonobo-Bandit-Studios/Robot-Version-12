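; BP_Gun is a gun pickup actor that the third-person player can fire.
; Overlapping its trigger zone sets the character's GunPickedup flag, which the end-overlap event leaves untouched.
; It enables its own input and handles Shoot, checking the character's current weapon and Holding state.
; Shots spawn a scaled-down BulletBP at the muzzle reference, aimed along the follow camera with an upward pitch offset.
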(event OnComponentBeginOverlap(TriggerZone)
  (params (OverlappedComponent :type Primitive%20Component%20Object%20Reference) (OtherActor :type Actor%20Object%20Reference) (OtherComp :type Primitive%20Component%20Object%20Reference) (OtherBodyIndex :type Integer) (bFromSweep :type Boolean) (SweepResult :type Hit%20Result%20Structure%20%28by%20ref%29))
  ;[1 1 1] Overlapping?
  (bind _asbp_third_person_character (Utilities|Casting|CastToBP_ThirdPersonCharacter OtherActor))
  (Variables|/Game/ThirdPerson/Blueprints/BP_ThirdPersonCharacter.BP_ThirdPersonCharacter_C|SetGunPickedup? _asbp_third_person_character true))

(event OnComponentEndOverlap(TriggerZone)
  (params (OverlappedComponent :type Primitive%20Component%20Object%20Reference) (OtherActor :type Actor%20Object%20Reference) (OtherComp :type Primitive%20Component%20Object%20Reference) (OtherBodyIndex :type Integer))
  ;[1 1 1] Overlapping?
)

(event EventBeginPlay
  (Input|EnableInput (Game|GetPlayerController 0)))

(event EventUpdateWeaponType
  (params (EWeaponType :type WeaponsEnum%20Enum :default "NewEnumerator0"))
  (Variables|Default|SetweaponType EWeaponType))

(event Input|ActionEvents|InputActionShoot
  (params (Key :type Key%20Structure :default "None"))
  (:Pressed
    (bind _asbp_third_person_character (Utilities|Casting|CastToBP_ThirdPersonCharacter (Game|GetPlayerCharacter 0)))
    (if (Utilities|Enum|Equal(Enum) (Variables|/Game/ThirdPerson/Blueprints/BP_ThirdPersonCharacter.BP_ThirdPersonCharacter_C|GetCurrentWeapon _asbp_third_person_character) "NewEnumerator0")
      (if (Variables|/Game/ThirdPerson/Blueprints/BP_ThirdPersonCharacter.BP_ThirdPersonCharacter_C|GetHolding? _asbp_third_person_character)
        (Game|SpawnActorfromClass "/Game/Pickup_Objs/BulletBP.BulletBP_C" (Math|Transform|MakeTransform (Transformation|GetWorldLocation (Variables|Default|GetBulletRef)) (Math|Rotator|MakeRotator (.roll (Transformation|GetWorldRotation (Variables|/Script/Robot_Protype_V3.Robot_Protype_V3Character|GetFollowCamera _asbp_third_person_character))) (+ (.pitch (Transformation|GetWorldRotation (Variables|/Script/Robot_Protype_V3.Robot_Protype_V3Character|GetFollowCamera _asbp_third_person_character))) 7.0) (.yaw (Transformation|GetWorldRotation (Variables|/Script/Robot_Protype_V3.Robot_Protype_V3Character|GetFollowCamera _asbp_third_person_character)))) "0.200000,0.200000,0.200000") "Undefined" "MultiplyWithRoot" 0 0)))))

(fn ConstructionScript)

(fn EssentialValues
  (return "0, 0, 0"))